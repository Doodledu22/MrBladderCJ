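; Master firework projectile actor that, once fired, flies with launch sound and trails, then explodes after random timed delays.
; Setup applies trail and burst particle templates and removes the unused second trail or smoke, with optional spiral using offset trails and actor spin.
; Tick adjusts velocity by curve until the burst and drives trail and burst colors through curve-based lerps, optionally ping-ponging.
; Explode stops trails and plays sound, then DelayExplode fires the burst and sets lifespan.
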(event `self.ReceiveBeginPlay`
  (bind (_randomscale_x _randomscale_y) (`KismetMathLibrary.BreakVector2D` (`self.RandomScale`)))
  ;[1 1 1] Set a relative rotation offset, and if spiral set location offset of the trails
  (`self.Setup`)
  (`SceneComponent.K2_SetRelativeRotation` (`self.FireWorksParticle`) (`KismetMathLibrary.MakeRotator` 0.0 0.0 (`KismetMathLibrary.RandomFloatInRange` -180.0 180.0)) false false)
  (`ParticleSystemComponent.SetColorParameter` (`self.FireWorksParticle`) "EColor" (`self.EndColor`))
  (`ParticleSystemComponent.SetColorParameter` (`self.FireWorksParticle`) "E2Color" (`self.End2Color`))
  (if (`self.bSpiral`)
    (`SceneComponent.K2_SetRelativeLocation` (`self.Trail`) (`KismetMathLibrary.MakeVector` (`self.SpiralOffset`)) false false)
    (`SceneComponent.K2_SetRelativeLocation` (`self.SecondTrail`) (`KismetMathLibrary.MakeVector` (* (`self.SpiralOffset`) -1.0)) false false))
  (`SceneComponent.SetRelativeScale3D` (`self.FireWorksParticle`) (`KismetMathLibrary.Conv_DoubleToVector` (`KismetMathLibrary.RandomFloatInRange` _randomscale_x _randomscale_y))))

(event `self.ReceiveTick`
  (params (DeltaSeconds :type "Float (single-precision)"))
  (bind (_initialvelocity_x _initialvelocity_y) (`KismetMathLibrary.BreakVector` (`self.InitialVelocity`)))
  (bind _projectilemovement (`self.ProjectileMovement`))
  ;[1 1 1] On tick.. Set delta, and if we're fired add to custom time, and check if we're not exploded, then update the velocity with a horizontal offset
  (bind _output_get (set `self.Delta` DeltaSeconds))
  (`self.HandleColor`)
  (if (`self.bFired`)
    (set `self.Time` (+ _output_get (`self.Time`)))
    (if (not (`self.bActualExplode`))
      (set `MovementComponent.Velocity` (+ (`MovementComponent.Velocity` _projectilemovement) (* (* (`KismetMathLibrary.Normal` (`KismetMathLibrary.MakeVector` _initialvelocity_x _initialvelocity_y (`KismetMathLibrary.Lerp` 0.0 (`self.FinalSpeed`) (`CurveFloat.GetFloatValue` (`self.Curve`) (`KismetMathLibrary.FClamp` (`self.Time`)))))) _output_get) (`self.HorizontalDrag`))) _projectilemovement)
      ;[1 1 1] On tick... add rotation offset
      (`self.K2_AddActorLocalRotation` (`KismetMathLibrary.MakeRotator` 0.0 0.0 (* (`self.SpiralRotSpeed`) (`self.Delta`)))))))

(fn `ConstructSetup`
  (bind _secondtrail (`self.SecondTrail`))
  ;[1 1 1] Construct setup to use smoke and if we're spiral or not
  (`|ExecutionSequence`
    (:`then_0`
      (if (not (`self.bSpiral`))
        (`/Engine/EditorBlueprintResources/StandardMacros.IsValid` _secondtrail
          (:`Is Valid`
            (`ActorComponent.K2_DestroyComponent` _secondtrail)))))
    (:`then_1`
      (if (`self.bUseSmoke`)
        (`ActorComponent.Activate` (`self.SmokeTrail`) false)
        (else
          (`ActorComponent.K2_DestroyComponent` (`self.SmokeTrail`)))))))

(fn `DelayExplode`
  (bind _smoketrail (`self.SmokeTrail`))
  ;[1 1 1] On actual explode, activate the firework and set the lifespan
  (set `self.bActualExplode` true)
  (`ActorComponent.Activate` (`self.FireWorksParticle`) true)
  (`self.SetLifeSpan` (`self.LifespanAfterExplode`))
  (`ActorComponent.Deactivate` (`self.ProjectileMovement`))
  (`/Engine/EditorBlueprintResources/StandardMacros.IsValid` _smoketrail
    (:`Is Valid`
      (`ActorComponent.Deactivate` _smoketrail))
    (:`Is Not Valid`
      _))
  (return))

(fn `Explode`
  (bind _smoke (`self.Smoke`))
  (bind (_randomdelayexplode_x _randomdelayexplode_y) (`KismetMathLibrary.BreakVector2D` (`self.RandomDelayExplode`)))
  ;[1 1 1] On explode, set ourselves to exploded and deactive trails, destroy the mesh and do a delayed explosion
  (set `self.bExploded` true)
  (`|ExecutionSequence`
    (:`then_0`
      (`ActorComponent.Deactivate` (`self.Trail`))
      (`/Engine/EditorBlueprintResources/StandardMacros.IsValid` (`self.SecondTrail`)
        (:`Is Valid`
          (`ActorComponent.Deactivate` (`self.SecondTrail`)))
        (:`Is Not Valid`
          _))
      (`KismetSystemLibrary.K2_SetTimer` null "DelayExplode" (`KismetMathLibrary.RandomFloatInRange` _randomdelayexplode_x _randomdelayexplode_y)))
    (:`then_1`
      (`/Engine/EditorBlueprintResources/StandardMacros.IsValid` _smoke
        (:`Is Valid`
          (`ActorComponent.Deactivate` _smoke))
        (:`Is Not Valid`
          _))
      (`GameplayStatics.PlaySoundAtLocation` (`self.ExplosionCue`) (`self.K2_GetActorLocation`) (struct) 1.0 1.0 0.0 "/Game/MFK/Sounds/FireworkAttenuation.FireworkAttenuation")
      (return))))

(fn `Fire`
  (params (Velocity :type "Vector Structure"))
  (bind _projectilemovement (`self.ProjectileMovement`))
  (bind (_explodetime_x _explodetime_y) (`KismetMathLibrary.BreakVector2D` (`self.ExplodeTime`)))
  ;[1 1 1] Set initial velocity
  (bind _output_get (set `self.InitialVelocity` (`KismetMathLibrary.MakeVector` (.x Velocity) (.y Velocity) (`self.FinalSpeed`))))
  ;[1 1 1] Set this as the velocity
  (set `MovementComponent.Velocity` _output_get _projectilemovement)
  ;[1 1 1] Active the smoke trail(s)
  (`ActorComponent.Activate` _projectilemovement true)
  (`ActorComponent.Activate` (`self.Trail`) true)
  (`/Engine/EditorBlueprintResources/StandardMacros.IsValid` (`self.SecondTrail`)
    (:`Is Valid`
      (`ActorComponent.Activate` (`self.SecondTrail`) true))
    (:`Is Not Valid`
      _))
  ;[1 1 1] Set the random explode time and set ourself to fired
  (`KismetSystemLibrary.K2_SetTimer` null "Explode" (`KismetMathLibrary.RandomFloatInRange` _explodetime_x _explodetime_y))
  (set `self.bFired` true)
  (`GameplayStatics.PlaySoundAtLocation` (`self.LaunchCue`) (`self.K2_GetActorLocation`) (struct) 1.0 1.0 0.0 "/Game/MFK/Sounds/FireworkAttenuation.FireworkAttenuation" "/Game/MFK/Sounds/NewSoundConcurrency.NewSoundConcurrency")
  (return))

(fn `GetFireworkParticle`
  (returns (FireworkParticle :type "ParticleSystem Object Reference"))
  ;[1 1 1] Get the firework particle
  (return (`self.FireworkParticle`)))

(fn `GetTrailParticle`
  (returns (TrailParticle :type "ParticleSystem Object Reference"))
  ;[1 1 1] Get the trail particke
  (return (`self.TrailParticle`)))

(fn `HandleColor`
  (bind _secondtrail (`self.SecondTrail`))
  (bind _returnvalue (`KismetMathLibrary.InverseLerp` 0.0 (`self.TrailColorOverTime`) (`self.BeforeExplodeTime`)))
  (bind _returnvalue_2 (`KismetMathLibrary.InverseLerp` 0.0 (`self.FirstColorOverTime`) (`self.AfterExplodeTime`)))
  ;[1 1 1] Handle trail color
  (`|ExecutionSequence`
    (:`then_0`
      (set `self.BeforeExplodeTime` (+ (`self.BeforeExplodeTime`) (`self.Delta`)))
      (set `self.TrailUseColor` (`KismetMathLibrary.LinearColorLerp` (`self.TrailColorStart`) (`self.TrailColorEnd`) (`KismetMathLibrary.FClamp` (`CurveFloat.GetFloatValue` (`self.TrailCurve`) (`KismetMathLibrary.FClamp` (select `bool` (`self.bForwardTrail`) :`false` (`KismetMathLibrary.Lerp` 1.0 0.0 _returnvalue) :`true` _returnvalue))))))
      (`ParticleSystemComponent.SetColorParameter` (`self.Trail`) "TColor" (`self.TrailUseColor`))
      (`/Engine/EditorBlueprintResources/StandardMacros.IsValid` _secondtrail
        (:`Is Valid`
          (`ParticleSystemComponent.SetColorParameter` _secondtrail "TColor" (`self.TrailUseColor`)))
        (:`Is Not Valid`
          _))
      (if (`self.bLoopTrailTime`)
        (if (> (`self.BeforeExplodeTime`) (`self.TrailColorOverTime`))
          (set `self.BeforeExplodeTime` 0.0)
          (set `self.bForwardTrail` (not (`self.bForwardTrail`)) :!label _label)
          (elif (<= (`self.BeforeExplodeTime`) 0.0)
            (goto _label)))))
    (:`then_1`
      ;[1 1 1] On explode... Do the after explode color lerp
      (if (`self.bActualExplode`)
        (set `self.AfterExplodeTime` (+ (`self.AfterExplodeTime`) (`self.Delta`)))
        (set `self.FirstUseColor` (`KismetMathLibrary.LinearColorLerp` (`self.FirstColorStart`) (`self.FirstColorEnd`) (`CurveFloat.GetFloatValue` (`self.FirstCurve`) (`KismetMathLibrary.FClamp` (select `bool` (`self.bForwardFirst`) :`false` (`KismetMathLibrary.Lerp` 1.0 0.0 _returnvalue_2) :`true` _returnvalue_2)))))
        (`ParticleSystemComponent.SetColorParameter` (`self.FireWorksParticle`) "FColor" (`self.FirstUseColor`))
        (if (`self.bLoopFirstTime`)
          (if (> (`self.AfterExplodeTime`) (`self.FirstColorOverTime`))
            (set `self.AfterExplodeTime` 0.0)
            (set `self.bForwardFirst` (not (`self.bForwardFirst`)) :!label _label_2)
            (return)
            (elif (<= (`self.AfterExplodeTime`) 0.0)
              (goto _label_2)
              (else
                _))))
        (return)
        (else
          (return))))))

(fn `Setup`
  ;[1 1 1] Setup the second trail if valid and set template of the trail
  (`/Engine/EditorBlueprintResources/StandardMacros.IsValid` (`self.SecondTrail`)
    (:`Is Valid`
      (`ParticleSystemComponent.SetTemplate` (`self.Trail`) (`self.GetTrailParticle`))
      (`ParticleSystemComponent.SetTemplate` (`self.SecondTrail`) (`self.GetTrailParticle`)))
    (:`Is Not Valid`
      _))
  (`ParticleSystemComponent.SetTemplate` (`self.FireWorksParticle`) (`self.GetFireworkParticle`))
  (`self.ConstructSetup`))

(fn `UserConstructionScript`
  ;[1 1 1] Set the templates of the particles and if not spiral, kill the second trail
  (`self.Setup`))