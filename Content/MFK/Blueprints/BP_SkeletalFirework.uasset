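; Skeletal firework Blueprint that bursts into an animated figure shaped by particles and sinking from the sky.
; On delayed explosion it spawns a SkeletalMeshActor at the shell, optionally with random yaw, sets its material, physics and animation.
; That actor feeds the particle system's "SKMesh_Surf" parameter as the emission surface.
; Tick then lerps it downward by a random distance, using FallCurve over the remaining lifespan.
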(event `self.ReceiveTick`
  (params (DeltaSeconds :type "Float (single-precision)"))
  ;[1 1 1] On tick and explode slowly move down
  (`parent.ReceiveTick` DeltaSeconds)
  (if (`self.bActualExplode`)
    (`self.K2_SetActorLocation` (`self.SkelMesh`) (`KismetMathLibrary.VLerp` (`self.Start`) (`self.Offset`) (`CurveFloat.GetFloatValue` (`self.FallCurve`) (`KismetMathLibrary.InverseLerp` (`self.LifespanAfterExplode`) 0.0 (`self.GetLifeSpan`)))) false false)))

(event `self.DelayExplode`
  (bind _bshouldrandomrot (`self.bShouldRandomRot`))
  ;[1 1 1] When explode create the skel mesh and set start and offset to go down
  (`parent.DelayExplode`)
  (set `self.bActualExplode` true)
  (bind _returnvalue (`|SpawnActorFromClass` "/Script/Engine.SkeletalMeshActor" (`KismetMathLibrary.MakeTransform` (`self.K2_GetActorLocation`) (select `bool` _bshouldrandomrot :`false` (`self.K2_GetActorRotation`) :`true` (`KismetMathLibrary.MakeRotator` 0.0 0.0 (* (`KismetMathLibrary.RandomFloatInRange` -180.0 180.0) (`KismetMathLibrary.Conv_IntToDouble` (`KismetMathLibrary.Conv_BoolToInt` _bshouldrandomrot))))) (1.0 1.0 1.0)) "AdjustIfPossibleButDontSpawnIfColliding" "OverrideRootScale")) ; Spawn the skeletal mesh actor at the locatin of the shell
  (set `self.SkelMesh` _returnvalue)
  (`PrimitiveComponent.SetSimulatePhysics` _returnvalue true) ; Turn on physics so the skeletal mesh actor falls. The rate is controlled by the Lineardampening property in the physics asset
  (bind _skeletalmeshcomponent (`SkeletalMeshActor.SkeletalMeshComponent` _returnvalue))
  (`PrimitiveComponent.SetMaterial` _skeletalmeshcomponent 0 (`self.SkeletalMaterial`)) ; Need to set the material to something clear
  (`SkinnedMeshComponent.SetSkinnedAssetAndUpdate` _skeletalmeshcomponent (`self.SkeletalMesh`) true) ; Set teh skeletal mesh to the one defined
  (`PrimitiveComponent.SetCollisionEnabled` _skeletalmeshcomponent "PhysicsOnly")
  (`ParticleSystemComponent.SetActorParameter` (`self.FireWorksParticle`) "SKMesh_Surf" (`self.SkelMesh`))
  (`SkeletalMeshComponent.PlayAnimation` _skeletalmeshcomponent (`self.AnimationSequence`) (`self.Loopanimation`))
  (set `self.Start` (`self.K2_GetActorLocation` (`self.SkelMesh`)))
  (set `self.Offset` (- (`self.Start`) (`KismetMathLibrary.MakeVector` 0.0 0.0 (`KismetMathLibrary.RandomFloatInRange` 6000.0 9000.0)))))

(fn `UserConstructionScript`
  ;[1 1 1] override
  (`parent.UserConstructionScript`))