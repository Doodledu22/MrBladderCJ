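; BP_Battery_Lines is a firework battery actor that lays out its base tubes in a rectangular grid.
; The construction script loops over YAmount columns and XAmount rows at Space intervals, adding an instanced static mesh to Battery for each cell.
; It also rebuilds FireWorksLoc with each cell's world position, found by rotating the local offset by the actor's rotation and adding its location.
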(fn `UserConstructionScript`
  (bind _space (`self.Space`))
  ;[1 1 1] Construct line array and crete instance static meshes for the firwork base
  (`KismetArrayLibrary.Array_Clear` (`self.FireWorksLoc`))
  (for _index (range 1 (+ (`self.XAmount`) 1))
    (for _index_2 (range 1 (+ (`self.YAmount`) 1))
      (bind _returnvalue (`KismetMathLibrary.MakeVector` (* (- _index_2 1) _space) (* (- _index 1) _space)))
      (`InstancedStaticMeshComponent.AddInstance` (`self.Battery`) (`KismetMathLibrary.MakeTransform` _returnvalue (struct) (1.0 1.0 1.0)))
      (`KismetArrayLibrary.Array_Add` (`self.FireWorksLoc`) (+ (`KismetMathLibrary.GreaterGreater_VectorRotator` _returnvalue (`self.K2_GetActorRotation`)) (`self.K2_GetActorLocation`))))))