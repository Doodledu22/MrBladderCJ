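; BP_Battery_Circle is a fireworks battery actor that lays out its battery pieces in a ring.
; The construction script spaces CircleAmount instances evenly at CircleSize radius by stepping yaw, adding each to the Battery instanced mesh in local space with no individual rotation.
; It also stores each point in FireWorksLoc as a world position, applying the actor's rotation and location but not its scale.
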(fn `UserConstructionScript`
  (bind _circleamount (`self.CircleAmount`))
  ;[1 1 1] Create a circular battery and store location
  (for _index (range _circleamount)
    (bind _returnvalue (* (`KismetMathLibrary.GetForwardVector` (`KismetMathLibrary.MakeRotator` 0.0 0.0 (* _index (/ 360.0 (`KismetMathLibrary.Conv_IntToDouble` _circleamount))))) (`self.CircleSize`)))
    (`InstancedStaticMeshComponent.AddInstance` (`self.Battery`) (`KismetMathLibrary.MakeTransform` _returnvalue))
    (`KismetArrayLibrary.Array_Add` (`self.FireWorksLoc`) (+ (`KismetMathLibrary.GreaterGreater_VectorRotator` _returnvalue (`self.K2_GetActorRotation`)) (`self.K2_GetActorLocation`)))))