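; Firework battery Blueprint that lays out instanced battery meshes as a grid of clusters, each cluster being a smaller grid.
; The Construction Script uses four nested loops over cluster and item counts, with separate spacing values, to add instances to the Battery component.
; For each instance it also appends the offset, rotated by the actor's rotation and shifted to its location, to FireWorksLoc as a world-space position.
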(fn `UserConstructionScript`
  (bind _space (`self.Space`))
  (bind _clusterspace (`self.ClusterSpace`))
  ;[1 1 1] Create the clusers and items in clusters. Also store location
  (for _index (range (`self.XAmount`))
    (for _index_2 (range (`self.YAmount`))
      (for _index_3 (range 1 (+ (`self.ClusterXAmount`) 1))
        (for _index_4 (range 1 (+ (`self.ClusterYAmount`) 1))
          (bind _returnvalue (+ (`KismetMathLibrary.MakeVector` (* _index_4 _clusterspace) (* _index_3 _clusterspace)) (`KismetMathLibrary.MakeVector` (* _index_2 _space) (* _index _space))))
          (`InstancedStaticMeshComponent.AddInstance` (`self.Battery`) (`KismetMathLibrary.MakeTransform` _returnvalue))
          (`KismetArrayLibrary.Array_Add` (`self.FireWorksLoc`) (+ (`KismetMathLibrary.GreaterGreater_VectorRotator` _returnvalue (`self.K2_GetActorRotation`)) (`self.K2_GetActorLocation`))))))))