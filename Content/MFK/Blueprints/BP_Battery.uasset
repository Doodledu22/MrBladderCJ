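; Firework battery actor that launches a sequence of fireworks from a list of locations after a startup delay, if active.
; A looping timer calls FireSingle, which spawns a firework at the next location using the actor's rotation with an offset, then fires it with a seeded random horizontal spread.
; When the list runs out, the timer stops, or the index resets to repeat the sequence up to a loop limit if looping is enabled.
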(event `self.ReceiveBeginPlay`
  (bind _initialdelay (`self.InitialDelay`))
  (if (`self.bDebugNoDelay`)
    (`KismetSystemLibrary.Delay` 0.05 :!label _label)
    (`self.StartFire`)
    (elif (> _initialdelay 0.0)
      (`KismetSystemLibrary.K2_SetTimer` null "StartFire" _initialdelay)
      (else
        (goto _label)))))

(fn `FireFirework`
  (params (Index :type Integer))
  (bind _horizontaloffset (`self.HorizontalOffset`))
  (bind _randstream (`self.RandStream`))
  (bind _returnvalue (`KismetArrayLibrary.Array_IsValidIndex` (`self.FireWorksLoc`) Index))
  (bind _returnvalue_2 (- _horizontaloffset (* _horizontaloffset 2.0)))
  ;[1 1 1] Fire firework but check for valid index and loop
  (if _returnvalue
    ;[1 1 1] Spawn the firework and fire it
    (bind _returnvalue_3 (`|SpawnActorFromClass` (`self.FireworkClass`) (`KismetMathLibrary.MakeTransform` (`KismetArrayLibrary.Array_Get` (`self.FireWorksLoc`) Index) (`KismetMathLibrary.ComposeRotators` (`self.K2_GetActorRotation`) (struct :`Yaw` -90.0))) "Undefined" "OverrideRootScale" null (`self.FireworkSpeed`)))
    (`/Engine/EditorBlueprintResources/StandardMacros.IsValid` _returnvalue_3
      (:`Is Valid`
        (`/Game/MFK/Blueprints/BP_MasterFirework.Fire` _returnvalue_3 (`KismetMathLibrary.MakeVector` (`KismetMathLibrary.RandomFloatInRangeFromStream` _returnvalue_2 _horizontaloffset _randstream) (`KismetMathLibrary.RandomFloatInRangeFromStream` _returnvalue_2 _horizontaloffset _randstream)))
        ;[1 1 1] Add to active index and check for a loop again
        (bind _output_get (set `self.ActiveIndex` (+ (`self.ActiveIndex`) 1)))
        (`self.LoopCheck` (not (`KismetArrayLibrary.Array_IsValidIndex` (`self.FireWorksLoc`) _output_get)))))
    (else
      (`self.LoopCheck` _returnvalue))))

(fn `FireSingle`
  ;[1 1 1] Fire a single firework
  ;[1 1 1] If we don't and we should loop then restart
  (if (<= (`KismetArrayLibrary.Array_Length` (`self.FireWorksLoc`)) (+ (`self.ActiveIndex`) 1))
    (if (not (`self.bShouldLoop`))
      (`KismetSystemLibrary.K2_ClearAndInvalidateTimerHandle` (`self.FireSingleTimer`))))
  ;[1 1 1] Fire Actual
  (`self.FireFirework` (`self.ActiveIndex`)))

(fn `LoopCheck`
  (params (IsNotValid :type Boolean))
  ;[1 1 1] Check for loops and if exceed loop count, stop the timer
  ;;[1 1 1] If we're not valid and we should loop
  (if (and (`self.bShouldLoop`) IsNotValid)
    ;;[1 1 1] Are we out of items?
    (if (<= (`self.LoopCount`) (`self.AmountOfLoops`))
      ;;[1 1 1] Yes? Reset values
      (set `self.ActiveIndex` 0)
      (set `self.LoopCount` (+ (`self.LoopCount`) 1))
      (bind _returnvalue (`KismetSystemLibrary.K2_SetTimer` null "FireSingle" (`self.DelayBetweenShots`) true))
      (set `self.FireSingleTimer` _returnvalue)
      (return)
      (else
        ;;[1 1 1] No? Cancel fire single timer
        (`KismetSystemLibrary.K2_ClearAndInvalidateTimerHandle` (`self.FireSingleTimer`))
        (return)))
    (else
      (return))))

(fn `StartFire`
  ;[1 1 1] Start the fire
  (if (`self.bActive`)
    (`self.FireSingle`)
    (bind _returnvalue (`KismetSystemLibrary.K2_SetTimer` null "FireSingle" (`KismetMathLibrary.FClamp` (`self.DelayBetweenShots`) 0.001 9999.0) true))
    (set `self.FireSingleTimer` _returnvalue)))

(fn `UserConstructionScript`)