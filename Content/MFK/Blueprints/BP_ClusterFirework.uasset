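; Cluster firework projectile, a child Blueprint that bursts into several particle effects when it explodes.
; The construction script spawns an inactive particle component per Cluster entry, optionally offset by a shared random yaw.
; DelayExplode activates the clusters, stops projectile movement, destroys the mesh and sets a lifespan.
; HandleColors drives particle color parameters with curve-based lerps for trails and exploded clusters, optionally looping in alternating directions; end colors are set at BeginPlay.
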(event `self.ReceiveBeginPlay`
  ;[1 1 1] On begin play set end and end 2 colors
  (`parent.ReceiveBeginPlay`)
  (for _array_element (`self.Clusters`)
    (`ParticleSystemComponent.SetColorParameter` _array_element "EColor" (`self.EndColor`))
    (`ParticleSystemComponent.SetColorParameter` _array_element "E2Color" (`self.End2Color`))))

(event `self.ReceiveTick`
  (params (DeltaSeconds :type "Float (single-precision)"))
  ;[1 1 1] Parent tick
  (`parent.ReceiveTick` DeltaSeconds))

(event `self.HandleColor`
  ;[1 1 1] Handle colors
  (`self.HandleColors`))

(event `self.DelayExplode`
  ;[1 1 1] On explode set clusters active and deactive movement
  (set `self.bActualExplode` true)
  (for _array_element (`self.Clusters`)
    (`ActorComponent.SetActive` _array_element true false))
  (`self.SetLifeSpan` (`self.LifespanAfterExplode`))
  (`ActorComponent.Deactivate` (`self.ProjectileMovement`))
  (`ActorComponent.K2_DestroyComponent` (`self.StaticMesh`)))

(fn `HandleColors`
  (bind _secondtrail (`self.SecondTrail`))
  (bind _returnvalue (`KismetMathLibrary.InverseLerp` 0.0 (`self.TrailColorOverTime`) (`self.BeforeExplodeTime`)))
  (bind _returnvalue_2 (`KismetMathLibrary.InverseLerp` 0.0 (`self.FirstColorOverTime`) (`self.AfterExplodeTime`)))
  ;[1 1 1] Handle trail color
  (`|ExecutionSequence`
    (:`then_0`
      (set `self.BeforeExplodeTime` (+ (`self.BeforeExplodeTime`) (`self.Delta`)))
      (set `self.TrailUseColor` (`KismetMathLibrary.LinearColorLerp` (`self.TrailColorStart`) (`self.TrailColorEnd`) (`KismetMathLibrary.FClamp` (`CurveFloat.GetFloatValue` (`self.TrailCurve`) (`KismetMathLibrary.FClamp` (select `bool` (`self.bForwardTrail`) :`false` (`KismetMathLibrary.Lerp` 1.0 0.0 _returnvalue) :`true` _returnvalue))))))
      (`ParticleSystemComponent.SetColorParameter` (`self.Trail`) "TColor" (`self.TrailUseColor`))
      (`/Engine/EditorBlueprintResources/StandardMacros.IsValid` _secondtrail
        (:`Is Valid`
          (`ParticleSystemComponent.SetColorParameter` _secondtrail "TColor" (`self.TrailUseColor`)))
        (:`Is Not Valid`
          _))
      (if (`self.bLoopTrailTime`)
        (if (> (`self.BeforeExplodeTime`) (`self.TrailColorOverTime`))
          (set `self.BeforeExplodeTime` 0.0)
          (set `self.bForwardTrail` (not (`self.bForwardTrail`)) :!label _label)
          (elif (<= (`self.BeforeExplodeTime`) 0.0)
            (goto _label)))))
    (:`then_1`
      ;[1 1 1] On explode... Do the after explode color lerp
      (if (`self.bActualExplode`)
        (set `self.AfterExplodeTime` (+ (`self.AfterExplodeTime`) (`self.Delta`)))
        (set `self.FirstUseColor` (`KismetMathLibrary.LinearColorLerp` (`self.FirstColorStart`) (`self.FirstColorEnd`) (`CurveFloat.GetFloatValue` (`self.FirstCurve`) (`KismetMathLibrary.FClamp` (select `bool` (`self.bForwardFirst`) :`false` (`KismetMathLibrary.Lerp` 1.0 0.0 _returnvalue_2) :`true` _returnvalue_2)))))
        (for _array_element (`self.Clusters`)
          (`ParticleSystemComponent.SetColorParameter` _array_element "FColor" (`self.FirstUseColor`)))
        (if (`self.bLoopFirstTime`)
          (if (> (`self.AfterExplodeTime`) (`self.FirstColorOverTime`))
            (set `self.AfterExplodeTime` 0.0)
            (set `self.bForwardFirst` (not (`self.bForwardFirst`)) :!label _label_2)
            (return)
            (elif (<= (`self.AfterExplodeTime`) 0.0)
              (goto _label_2)
              (else
                _))))
        (return)
        (else
          (return))))))

(fn `UserConstructionScript`
  (locals (RandomRot :type "Rotator Structure"))
  (set `local.RandomRot` (`KismetMathLibrary.MakeRotator` 0.0 0.0 (.yaw (`KismetMathLibrary.RandomRotator` false))))
  (for _array_element (`self.Cluster`)
    (bind (_particles _rotation) (break `/Game/MFK/Blueprints/Structs/ClusterStruct` _array_element))
    (bind _returnvalue (`AddComponent|ParticleSystemComponent_0` :`RelativeTransform` (`KismetMathLibrary.MakeTransform` (0.0 0.0 0.0) (`KismetMathLibrary.ComposeRotators` _rotation (select `bool` (`self.bUseRandomRot`) :`true` (`local.RandomRot`))))))
    (`ParticleSystemComponent.SetTemplate` _returnvalue _particles)
    (`KismetArrayLibrary.Array_Add` (`self.Clusters`) _returnvalue)
    (`ActorComponent.SetActive` _returnvalue false false))
  (`ParticleSystemComponent.SetTemplate` (`self.Trail`) (`self.GetTrailParticle`))
  (`ParticleSystemComponent.SetTemplate` (`self.SecondTrail`) (`self.GetTrailParticle`))
  (`ParticleSystemComponent.SetTemplate` (`self.FireWorksParticle`) null)
  (`self.ConstructSetup`))