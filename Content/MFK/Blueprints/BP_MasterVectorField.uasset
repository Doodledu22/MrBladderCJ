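; BP_MasterVectorField is a base Blueprint that configures a vector field component from exposed settings.
; Its construction script applies the tightness and intensity to the component.
; It then sets the component's relative rotation to a random yaw drawn from a random stream, keeping pitch and roll at zero, so the seed controls the orientation.
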(fn `UserConstructionScript`
  ;[1 1 1] Set the vector field settings
  (set `VectorFieldComponent.Tightness` (`self.Tightness`) (`self.VectorField`))
  (`VectorFieldComponent.SetIntensity` (`self.VectorField`) (`self.Intensity`))
  (`SceneComponent.K2_SetRelativeRotation` (`self.VectorField`) (`KismetMathLibrary.MakeRotator` 0.0 0.0 (.yaw (`KismetMathLibrary.RandomRotatorFromStream` false (`self.RandomStream`)))) false false))