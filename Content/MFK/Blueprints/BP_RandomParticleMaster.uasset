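; BP_RandomParticleMaster is a lookup Blueprint that supplies random particle effects for fireworks and their trails.
; GetTrailParticle returns a random entry from the RandomTrails array, and GetFireworkParticle does the same from RandomParticles.
; It has no active runtime logic of its own: the event graph holds only disabled default events and the construction script just calls its parent.
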(fn `GetFireworkParticle`
  (returns (FireworkParticle :type "ParticleSystem Object Reference"))
  (bind _randomparticles (`self.RandomParticles`))
  ;[1 1 1] Get random particle
  (return (`KismetArrayLibrary.Array_Get` _randomparticles (`KismetMathLibrary.RandomInteger` (`KismetArrayLibrary.Array_Length` _randomparticles)))))

(fn `GetTrailParticle`
  (returns (TrailParticle :type "ParticleSystem Object Reference"))
  (bind _randomtrails (`self.RandomTrails`))
  ;[1 1 1] Get random particle
  (return (`KismetArrayLibrary.Array_Get` _randomtrails (`KismetMathLibrary.RandomInteger` (`KismetArrayLibrary.Array_Length` _randomtrails)))))

(fn `UserConstructionScript`
  ;[1 1 1] override
  (`parent.UserConstructionScript`))