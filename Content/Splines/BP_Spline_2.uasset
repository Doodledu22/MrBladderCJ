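; BP_Spline_2 is an actor that moves its Character component along its Spline in a continuous loop.
; Each Tick advances the travelled distance by SplineSpeed scaled by delta time, then applies the spline's local-space location and rotation at that distance as Character's relative transform, preserving its scale.
; When the distance exceeds the spline length, it resets to zero and the run starts over.
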(event `self.ReceiveTick`
  (params (DeltaSeconds :type "Float (single-precision)"))
  (bind (_returnvalue_location _returnvalue_rotation) (`KismetMathLibrary.BreakTransform` (`SplineComponent.GetTransformAtDistanceAlongSpline` (`self.Spline`) (`self.Distance Along Spline`) "Local" false)))
  (set `self.Distance Along Spline` (+ (* DeltaSeconds (`self.Spline Speed`)) (`self.Distance Along Spline`)))
  (`SceneComponent.K2_SetRelativeTransform` (`self.Character`) (`KismetMathLibrary.MakeTransform` _returnvalue_location _returnvalue_rotation (`SceneComponent.RelativeScale3D` (`self.Character`))) false false)
  (if (> (`self.Distance Along Spline`) (`SplineComponent.GetSplineLength` (`self.Spline`)))
    (set `self.Distance Along Spline` 0.0)))

(fn `UserConstructionScript`)