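; Potion bottle actor with a configurable base mesh, inner and outer liquid meshes, and a lid, faking sloshing liquid through materials.
; Construction assigns meshes, materials and dynamic instances; BeginPlay recreates the liquid and lid instances.
; Tick turns base-mesh movement and rotation deltas into smoothed Distortion and X/Y Sine parameters, with movement-scaled smoothing when physics is off.
; Tick also reapplies fill amount, lid opacity and physics simulation every frame.
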(event `self.ReceiveBeginPlay`
  (bind _sm_potion2_base (`self.SM_Potion2_Base`))
  (bind (_relativerotation_roll _relativerotation_pitch _relativerotation_yaw) (`KismetMathLibrary.BreakRotator` (`SceneComponent.RelativeRotation` _sm_potion2_base)))
  ;[0 1 0.3855] Store Initial Position, Rotation and create Dynamic Material instance
  (set `self.Old Position` (`SceneComponent.RelativeLocation` _sm_potion2_base))
  (set `self.Old Rotation` (`KismetMathLibrary.MakeVector` _relativerotation_roll _relativerotation_pitch _relativerotation_yaw))
  (`self.Set Potion Type`))

(event `self.ReceiveTick`
  (params (DeltaSeconds :type "Float (single-precision)"))
  (bind _dmi_inner_liquid (`self.DMI_Inner_Liquid`))
  (bind _delta_seconds (`self.Delta Seconds`))
  (bind _delta_seconds_2 (`self.Delta Seconds`))
  (bind _delta_seconds_3 (`self.Delta Seconds`))
  (bind _sm_potion2_base (`self.SM_Potion2_Base`))
  (bind _sm_potion2_base_2 (`self.SM_Potion2_Base`))
  (bind (_relativelocation_x _relativelocation_y) (`KismetMathLibrary.BreakVector` (`SceneComponent.RelativeLocation` _sm_potion2_base_2)))
  (bind (_relativerotation_roll _relativerotation_pitch) (`KismetMathLibrary.BreakRotator` (`SceneComponent.RelativeRotation` _sm_potion2_base_2)))
  (bind _relativelocation (`SceneComponent.RelativeLocation` _sm_potion2_base))
  (bind (_relativerotation_roll_2 _relativerotation_pitch_2 _relativerotation_yaw) (`KismetMathLibrary.BreakRotator` (`SceneComponent.RelativeRotation` _sm_potion2_base)))
  (bind _returnvalue (`KismetMathLibrary.MakeVector` _relativerotation_roll_2 _relativerotation_pitch_2 _relativerotation_yaw))
  (bind _returnvalue_2 (- _relativelocation_y (.y (`self.Old Position`))))
  (bind _returnvalue_3 (- _relativelocation_x (.x (`self.Old Position`))))
  (bind _returnvalue_4 (- _relativerotation_pitch (.y (`self.Old Rotation`))))
  (bind _returnvalue_5 (- _relativerotation_roll (.x (`self.Old Rotation`))))
  (set `self.Delta Seconds` DeltaSeconds)
  (`|ExecutionSequence`
    (:`then_0`
      ;[0 0.2066 1] Set Distortion amount based on Movemnt and Rotation
      (`/Engine/EditorBlueprintResources/StandardMacros.IsValid` (`self.DMI_Inner_Liquid`)
        (:`Is Valid`
          (`/Engine/EditorBlueprintResources/StandardMacros.IsValid` (`self.DMI_Outer_Liquid`)
            (:`Is Valid`
              (bind _output_get (set `self.Current Distortion Amount` (`KismetMathLibrary.FInterpTo` (`self.Current Distortion Amount`) (`KismetMathLibrary.FClamp` (+ (/ (/ (`KismetMathLibrary.VSize` (- _relativelocation (`self.Old Position`))) _delta_seconds_2) 250.0) (/ (/ (`KismetMathLibrary.VSize` (- _returnvalue (`self.Old Rotation`))) _delta_seconds_2) 5.0)) 0.0 2.0) (`self.Delta Seconds`) 1.0)))
              (`MaterialInstanceDynamic.SetScalarParameterValue` (`self.DMI_Inner_Liquid`) "Distortion Amount" _output_get)
              (`MaterialInstanceDynamic.SetScalarParameterValue` (`self.DMI_Outer_Liquid`) "Distortion Amount" _output_get)
              (`MaterialInstanceDynamic.SetScalarParameterValue` (`self.DMI Lid`) "Distortion Amount" _output_get)
              (bind _output_get_2 (set `self.Current X Sine` (`KismetMathLibrary.FInterpTo` (`self.Current X Sine`) (`KismetMathLibrary.FClamp` (+ (/ (/ _returnvalue_3 _delta_seconds_3) 250.0) (/ (/ _returnvalue_4 _delta_seconds) 10.0)) -2.0 2.0) (`self.Delta Seconds`) (`KismetMathLibrary.SelectFloat` 1.0 (`KismetMathLibrary.FClamp` (* (`KismetMathLibrary.Abs` (+ _returnvalue_3 _returnvalue_4)) 5.0) 1.0 50.0) (`self.Simulate Physics`)))))
              (`MaterialInstanceDynamic.SetScalarParameterValue` _dmi_inner_liquid "X Sine" _output_get_2)
              (`MaterialInstanceDynamic.SetScalarParameterValue` (`self.DMI_Outer_Liquid`) "X Sine" _output_get_2)
              (`MaterialInstanceDynamic.SetScalarParameterValue` (`self.DMI Lid`) "X Sine" _output_get_2)
              (bind _output_get_3 (set `self.Current Y sine` (`KismetMathLibrary.FInterpTo` (`self.Current Y sine`) (`KismetMathLibrary.FClamp` (+ (/ (/ _returnvalue_2 _delta_seconds_3) 250.0) (/ (/ _returnvalue_5 _delta_seconds) 10.0)) -2.0 2.0) (`self.Delta Seconds`) (`KismetMathLibrary.SelectFloat` 1.0 (`KismetMathLibrary.FClamp` (* (`KismetMathLibrary.Abs` (+ _returnvalue_2 _returnvalue_5)) 5.0) 1.0 50.0) (`self.Simulate Physics`)))))
              (`MaterialInstanceDynamic.SetScalarParameterValue` _dmi_inner_liquid "Y Sine" _output_get_3)
              (`MaterialInstanceDynamic.SetScalarParameterValue` (`self.DMI Lid`) "Y Sine" _output_get_3)
              (`MaterialInstanceDynamic.SetScalarParameterValue` (`self.DMI_Outer_Liquid`) "Y Sine" _output_get_3)
              (set `self.Old Position` _relativelocation)
              (set `self.Old Rotation` _returnvalue))))))
    (:`then_1`
      ;[0 1 0.4804] Fill Amount
      (`MaterialInstanceDynamic.SetScalarParameterValue` (`self.DMI_Inner_Liquid`) "Fill Amount" (`self.Fill Amount`))
      (`MaterialInstanceDynamic.SetScalarParameterValue` (`self.DMI_Outer_Liquid`) "Fill Amount" (`self.Fill Amount`))
      (`MaterialInstanceDynamic.SetScalarParameterValue` (`self.DMI Lid`) "Fill Amount" (`self.Fill Amount`))
      (`MaterialInstanceDynamic.SetScalarParameterValue` (`self.DMI Lid`) "Opacity" (`KismetMathLibrary.Conv_BoolToDouble` (`self.Lid`)))
      (`PrimitiveComponent.SetSimulatePhysics` (`self.SM_Potion2_Base`) (`self.Simulate Physics`)))))

(event `Set Potion Type`
  ;[0 0.537 1] Set Potion Type
  (bind _returnvalue (`PrimitiveComponent.CreateDynamicMaterialInstance` (`self.SM_Potion2_Inner`) 0 (`self.Inner Liquid Material`) "None"))
  (set `self.DMI_Inner_Liquid` _returnvalue)
  (bind _returnvalue_2 (`PrimitiveComponent.CreateDynamicMaterialInstance` (`self.SM_Potion2_Outer`) 0 (`self.Outer Liquid Material`) "None"))
  (set `self.DMI_Outer_Liquid` _returnvalue_2)
  (bind _returnvalue_3 (`PrimitiveComponent.CreateDynamicMaterialInstance` (`self.SM_Potion2_Base`) (`KismetMathLibrary.Conv_BoolToInt` (`self.Invert Glass/Lid Material Index`)) (`self.Lid Material`) "None"))
  (set `self.DMI Lid` _returnvalue_3))

(event `Physics`
  (params (`bSimulate Physics` :type Boolean))
  ;[0.9893 1 0] Physics
  (`PrimitiveComponent.SetSimulatePhysics` (`self.SM_Potion2_Base`) `bSimulate Physics`))

(fn `UserConstructionScript`
  (bind _sm_potion2_base (`self.SM_Potion2_Base`))
  ;[0 1 0.0504] Cork Opacity and Fill Amount
  (`StaticMeshComponent.SetStaticMesh` (`self.SM_Potion2_Base`) (`self.Base Mesh`))
  (`StaticMeshComponent.SetStaticMesh` (`self.SM_Potion2_Inner`) (`self.Inner Liquid Mesh`))
  (`StaticMeshComponent.SetStaticMesh` (`self.SM_Potion2_Outer`) (`self.Outer Liquid Mesh`))
  (bind _returnvalue (`PrimitiveComponent.CreateDynamicMaterialInstance` (`self.SM_Potion2_Inner`) 0 (`self.Inner Liquid Material`) "None"))
  (set `self.DMI_Inner_Liquid` _returnvalue)
  (bind _returnvalue_2 (`PrimitiveComponent.CreateDynamicMaterialInstance` (`self.SM_Potion2_Outer`) 0 (`self.Outer Liquid Material`) "None"))
  (set `self.DMI_Outer_Liquid` _returnvalue_2)
  (bind _returnvalue_3 (`PrimitiveComponent.CreateDynamicMaterialInstance` (`self.SM_Potion2_Base`) (`KismetMathLibrary.Conv_BoolToInt` (`self.Invert Glass/Lid Material Index`)) (`self.Lid Material`) "None"))
  (bind _output_get (set `self.DMI Lid` _returnvalue_3))
  (`MaterialInstanceDynamic.SetScalarParameterValue` _output_get "Opacity" (`KismetMathLibrary.Conv_BoolToDouble` (`self.Lid`)))
  (`MaterialInstanceDynamic.SetScalarParameterValue` (`self.DMI_Inner_Liquid`) "Fill Amount" (`self.Fill Amount`))
  (`MaterialInstanceDynamic.SetScalarParameterValue` (`self.DMI_Outer_Liquid`) "Fill Amount" (`self.Fill Amount`))
  (`MaterialInstanceDynamic.SetScalarParameterValue` (`self.DMI Lid`) "Fill Amount" (`self.Fill Amount`))
  (`PrimitiveComponent.SetCastShadow` _sm_potion2_base (`self.Cast Shadow`))
  (`PrimitiveComponent.SetSimulatePhysics` _sm_potion2_base (`self.Simulate Physics`))
  (`PrimitiveComponent.CreateDynamicMaterialInstance` (`self.SM_Potion2_Base`) (`KismetMathLibrary.SelectInt` 0 1 (`self.Invert Glass/Lid Material Index`)) (`self.Glass Material`) "None"))