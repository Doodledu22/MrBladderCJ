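; BP_Potion_Child is a potion bottle variant meant to run as a child actor of the ALS_AnimMan character.
; On BeginPlay it casts its parent actor to that character and caches it as a player reference.
; Its updateFillAmount event integrates fill speed minus overflow over frame time, clamps the fill to a normalized range, and reports it to the character through OnFluidFillUpdate.
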(event `self.ReceiveBeginPlay`
  (`parent.ReceiveBeginPlay`)
  (bind _asals_anim_man_character_bp (cast `/Game/AdvancedLocomotionV4/Blueprints/CharacterLogic/ALS_AnimMan_CharacterBP` (`self.GetParentActor`)))
  (set `self.playerRef` _asals_anim_man_character_bp))

(event `self.ReceiveTick`
  (params (DeltaSeconds :type "Float (single-precision)"))
  (`parent.ReceiveTick` DeltaSeconds))

(event `updateFillAmount`
  (params (overflowAmount :type "Float (double-precision)"))
  (bind _output_get (set `self.Fill Amount` (`KismetMathLibrary.FClamp` (+ (* (- (`self.fillSpeed`) overflowAmount) (`GameplayStatics.GetWorldDeltaSeconds`)) (`self.Fill Amount`)))))
  (`/Game/AdvancedLocomotionV4/Blueprints/CharacterLogic/ALS_AnimMan_CharacterBP.onFluidFillUpdate` (`self.playerRef`) _output_get))

(fn `UserConstructionScript`
  (`parent.UserConstructionScript`))