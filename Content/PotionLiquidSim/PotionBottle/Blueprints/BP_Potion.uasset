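; Potion bottle actor that fakes sloshing liquid through material parameters, with configurable mesh, materials, fill amount, lid visibility, shadow and physics.
; The construction script and SetPotionType create dynamic liquid and lid materials, though SetPotionType uses hardcoded slot indices.
; Tick converts the bottle's per-frame movement and rotation into smoothed distortion and X/Y sine values for both materials.
; Tick also reapplies fill, lid opacity and physics simulation every frame.
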(event `self.ReceiveBeginPlay`
  (bind _sm_bottle (`self.SM_Bottle`))
  (bind (_relativerotation_roll _relativerotation_pitch _relativerotation_yaw) (`KismetMathLibrary.BreakRotator` (`SceneComponent.RelativeRotation` _sm_bottle)))
  ;[0.373 1 0] Store Initial Position, Rotation and create Dynamic Material instance
  (set `self.Old Position` (`SceneComponent.RelativeLocation` _sm_bottle))
  (set `self.Old Rotation` (`KismetMathLibrary.MakeVector` _relativerotation_roll _relativerotation_pitch _relativerotation_yaw))
  (`self.Set Potion Type`))

(event `self.ReceiveTick`
  (params (DeltaSeconds :type "Float (single-precision)"))
  (bind _delta_seconds (`self.Delta Seconds`))
  (bind _delta_seconds_2 (`self.Delta Seconds`))
  (bind _dmi_liquid_ (`self.DMI Liquid `))
  (bind _delta_seconds_3 (`self.Delta Seconds`))
  (bind _sm_bottle (`self.SM_Bottle`))
  (bind _sm_bottle_2 (`self.SM_Bottle`))
  (bind (_relativelocation_x _relativelocation_y) (`KismetMathLibrary.BreakVector` (`SceneComponent.RelativeLocation` _sm_bottle)))
  (bind (_relativerotation_roll _relativerotation_pitch) (`KismetMathLibrary.BreakRotator` (`SceneComponent.RelativeRotation` _sm_bottle)))
  (bind _relativelocation (`SceneComponent.RelativeLocation` _sm_bottle_2))
  (bind (_relativerotation_roll_2 _relativerotation_pitch_2 _relativerotation_yaw) (`KismetMathLibrary.BreakRotator` (`SceneComponent.RelativeRotation` _sm_bottle_2)))
  (bind _returnvalue (`KismetMathLibrary.MakeVector` _relativerotation_roll_2 _relativerotation_pitch_2 _relativerotation_yaw))
  (bind _returnvalue_2 (- _relativelocation_y (.y (`self.Old Position`))))
  (bind _returnvalue_3 (- _relativelocation_x (.x (`self.Old Position`))))
  (bind _returnvalue_4 (- _relativerotation_pitch (.y (`self.Old Rotation`))))
  (bind _returnvalue_5 (- _relativerotation_roll (.x (`self.Old Rotation`))))
  (set `self.Delta Seconds` DeltaSeconds)
  (`|ExecutionSequence`
    (:`then_0`
      ;[0.1505 0 1] Set Distortion amount based on Movemnt and Rotation
      (`/Engine/EditorBlueprintResources/StandardMacros.IsValid` _dmi_liquid_
        (:`Is Valid`
          (bind _output_get (set `self.Current Distortion Amount` (`KismetMathLibrary.FInterpTo` (`self.Current Distortion Amount`) (`KismetMathLibrary.FClamp` (+ (/ (/ (`KismetMathLibrary.VSize` (- _relativelocation (`self.Old Position`))) _delta_seconds_2) 250.0) (/ (/ (`KismetMathLibrary.VSize` (- _returnvalue (`self.Old Rotation`))) _delta_seconds_2) 5.0)) 0.0 2.0) (`self.Delta Seconds`) 1.0)))
          (`MaterialInstanceDynamic.SetScalarParameterValue` _dmi_liquid_ "Distortion Amount" _output_get)
          (`MaterialInstanceDynamic.SetScalarParameterValue` (`self.DMI Lid`) "Distortion Amount" _output_get)
          (bind _output_get_2 (set `self.Current X Sine` (`KismetMathLibrary.FInterpTo` (`self.Current X Sine`) (`KismetMathLibrary.FClamp` (+ (/ (/ _returnvalue_3 _delta_seconds_3) 250.0) (/ (/ _returnvalue_4 _delta_seconds) 10.0)) -2.0 2.0) (`self.Delta Seconds`) (`KismetMathLibrary.SelectFloat` 1.0 (`KismetMathLibrary.FClamp` (* (`KismetMathLibrary.Abs` (+ _returnvalue_3 _returnvalue_4)) 5.0) 1.0 50.0) (`self.Simulate Physics`)))))
          (`MaterialInstanceDynamic.SetScalarParameterValue` (`self.DMI Lid`) "X Sine" _output_get_2)
          (`MaterialInstanceDynamic.SetScalarParameterValue` (`self.DMI Liquid `) "X Sine" _output_get_2)
          (bind _output_get_3 (set `self.Current Y sine` (`KismetMathLibrary.FInterpTo` (`self.Current Y sine`) (`KismetMathLibrary.FClamp` (+ (/ (/ _returnvalue_2 _delta_seconds_3) 250.0) (/ (/ _returnvalue_5 _delta_seconds) 10.0)) -2.0 2.0) (`self.Delta Seconds`) (`KismetMathLibrary.SelectFloat` 1.0 (`KismetMathLibrary.FClamp` (* (`KismetMathLibrary.Abs` (+ _returnvalue_2 _returnvalue_5)) 5.0) 1.0 50.0) (`self.Simulate Physics`)))))
          (`MaterialInstanceDynamic.SetScalarParameterValue` (`self.DMI Liquid `) "Y Sine" _output_get_3)
          (`MaterialInstanceDynamic.SetScalarParameterValue` (`self.DMI Lid`) "Y Sine" _output_get_3)
          (set `self.Old Position` _relativelocation)
          (set `self.Old Rotation` _returnvalue))))
    (:`then_1`
      ;[0 0.6972 1] Fill Amount
      (`MaterialInstanceDynamic.SetScalarParameterValue` (`self.DMI Liquid `) "Fill Amount" (`self.Fill Amount`))
      (`MaterialInstanceDynamic.SetScalarParameterValue` (`self.DMI Lid`) "Fill Amount" (`self.Fill Amount`))
      (`MaterialInstanceDynamic.SetScalarParameterValue` (`self.DMI Lid`) "Opacity" (`KismetMathLibrary.Conv_BoolToDouble` (`self.Lid`)))
      (`PrimitiveComponent.SetSimulatePhysics` (`self.SM_Bottle`) (`self.Simulate Physics`)))))

(event `Set Potion Type`
  ;[0 1 0.1875] Set Potion Type
  (bind _returnvalue (`PrimitiveComponent.CreateDynamicMaterialInstance` (`self.SM_Bottle`) 0 (`self.Potion Material`) "None"))
  (set `self.DMI Liquid ` _returnvalue)
  (bind _returnvalue_2 (`PrimitiveComponent.CreateDynamicMaterialInstance` (`self.SM_Bottle`) 2 (`self.Lid Material`) "None"))
  (set `self.DMI Lid` _returnvalue_2))

(event `Physics`
  (params (`bSimulate Physics` :type Boolean))
  ;[0.9893 1 0] Physics
  (`PrimitiveComponent.SetSimulatePhysics` (`self.SM_Bottle`) `bSimulate Physics`))

(fn `UserConstructionScript`
  ;[0 1 0.07192] Cork Opoacity and Fill Amount
  (`StaticMeshComponent.SetStaticMesh` (`self.SM_Bottle`) (`self.Static Mesh`))
  (`PrimitiveComponent.CreateDynamicMaterialInstance` (`self.SM_Bottle`) (`self.Glass Material Index`) (`self.Glass Material`) "None")
  (bind _returnvalue (`PrimitiveComponent.CreateDynamicMaterialInstance` (`self.SM_Bottle`) (`self.Liquid Material Index`) (`self.Potion Material`) "None"))
  (bind _output_get (set `self.DMI Liquid ` _returnvalue))
  (bind _returnvalue_2 (`PrimitiveComponent.CreateDynamicMaterialInstance` (`self.SM_Bottle`) (`self.Lid Material Index`) (`self.Lid Material`) "None"))
  (bind _output_get_2 (set `self.DMI Lid` _returnvalue_2))
  (`MaterialInstanceDynamic.SetScalarParameterValue` _output_get_2 "Opacity" (`KismetMathLibrary.Conv_BoolToDouble` (`self.Lid`)))
  (`MaterialInstanceDynamic.SetScalarParameterValue` _output_get_2 "Fill Amount" (`self.Fill Amount`))
  (`MaterialInstanceDynamic.SetScalarParameterValue` _output_get "Fill Amount" (`self.Fill Amount`))
  (`PrimitiveComponent.SetCastShadow` (`self.SM_Bottle`) (`self.Cast Shadow`))
  (`PrimitiveComponent.SetSimulatePhysics` (`self.SM_Bottle`) (`self.Simulate Physics`)))